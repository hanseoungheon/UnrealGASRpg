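; BP_ABPC is a possessable character Blueprint in ArenaBattleGAS that owns the player HUD and reacts to game clear.
; On possession, it creates WBP_HUD for player controllers and listens for the Event.Game.Cleared gameplay tag on its Ability System Component.
; A change to that tag updates the HUD and activates the GameCleared component.
; A PlayerDeath handler sets IsDeath, but its binding to Event.Gimmick.Death never runs.
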(event Custom|OnGamePlay%20TargetChangeBP
  (params (Tag :type Gameplay%20Tag%20Structure%20%28by%20ref%29) (TagCount :type Integer))
  (Default|SetGameCleared (Variables|Default|GetHUDWidget))
  (Components|Activation|Activate (Variables|Default|GetGameCleared) false))

(event Custom|Player%20Death
  (params (Tag :type Gameplay%20Tag%20Structure%20%28by%20ref%29) (TagCount :type Integer))
  (Variables|Default|SetIsDeath true))

(event EventBeginPlay)

(event EventPossessed
  (params (NewController :type Controller%20Object%20Reference))
  (Utilities|FlowControl|Sequence
    (:then_0
      (if (Class|Controller|IsPlayerController NewController)
        (bind _returnvalue (UserInterface|CreateWidget "/Game/ArenaBattleGAS/UI/WBP_HUD.WBP_HUD_C"))
        (bind _output_get (Variables|Default|SetHUDWidget _returnvalue))
        (UserInterface|Viewport|AddtoViewport _output_get 0)))
    (:then_1
      (GameplayTags|BindEventWrappertoGameplayTagChanged (Variables|Default|GetASC) "(TagName=\"Event.Game.Cleared\")" (delegate Custom|OnGamePlay%20TargetChangeBP)))))

(fn ConstructionScript)